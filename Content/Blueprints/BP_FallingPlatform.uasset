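; Falling platform actor that drops shortly after the third-person character steps on it, then returns to its original spot and re-arms.
; A trigger box overlap while ready starts a delay, then physics simulation lets the platform fall for a set duration.
; Reset stops physics and a Timeline lerps the fallen transform back to the one saved at BeginPlay.
; Each phase swaps the platform's material and prints a debug message.
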(event OnComponentBeginOverlap(BoxTrigger)
  (params (OverlappedComponent :type Primitive%20Component%20Object%20Reference) (OtherActor :type Actor%20Object%20Reference) (OtherComp :type Primitive%20Component%20Object%20Reference) (OtherBodyIndex :type Integer) (bFromSweep :type Boolean) (SweepResult :type Hit%20Result%20Structure%20%28by%20ref%29))
  (Development|PrintString "Something is Standing on Me!")
  (if (Variables|Default|GetisReady)
    (Utilities|Casting|CastToBP_ThirdPersonCharacter OtherActor)
    (CallFunction|Activate)))

(event Custom|Activate
  (Variables|Default|SetisReady false)
  (Development|PrintString "Countdown Starting Now!")
  (Rendering|Material|SetMaterial (Variables|Default|GetPlatform) 0 "/Game/Materials/MI_ActivePlatform.MI_ActivePlatform")
  (Utilities|FlowControl|Delay (Variables|PlatformSettings|GetFall%20Delay%20Duration))
  (CallFunction|Falling))

(event Custom|Falling
  (Development|PrintString "Fallingggg!!!")
  (Rendering|Material|SetMaterial (Variables|Default|GetPlatform) 0 "/Game/Materials/MI_FallingPlatform.MI_FallingPlatform")
  (Physics|SetSimulatePhysics (Variables|Default|GetPlatform) true)
  (Utilities|FlowControl|Delay (Variables|PlatformSettings|GetFall%20Duration))
  (CallFunction|Reset))

(event Custom|Reset
  (Development|PrintString "Resetting the Platfrom!")
  (Rendering|Material|SetMaterial (Variables|Default|GetPlatform) 0 "/Game/Materials/MI_ResettingPlatform.MI_ResettingPlatform")
  (Physics|SetSimulatePhysics (Variables|Default|GetPlatform) false)
  (Variables|Default|SetFallen%20Transform (Transformation|GetWorldTransform (Variables|Default|GetPlatform)))
  (bind _newtrack_0 (Timeline|GoBackToStartTransfrom PlayFromStart)
    (:Update
      (Transformation|SetWorldTransform (Variables|Default|GetPlatform) (Math|Transform|Lerp(Transform) (Variables|Default|GetFallen%20Transform) (Variables|Default|GetStarting%20transform) _newtrack_0) false false))
    (:Finished
      (Variables|Default|SetisReady true)
      (Rendering|Material|SetMaterial (Variables|Default|GetPlatform) 0 "/Game/Materials/MI_ReadyPlatform.MI_ReadyPlatform"))))

(event EventBeginPlay
  (Variables|Default|SetStarting%20transform (Transformation|GetWorldTransform (Variables|Default|GetPlatform))))

(event Collision|EventActorBeginOverlap
  (params (OtherActor :type Actor%20Object%20Reference)))

(event EventTick
  (params (DeltaSeconds :type Float%20%28single-precision%29)))

(fn ConstructionScript)