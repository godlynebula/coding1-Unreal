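; Elevator actor that moves a platform from a Start to an End transform when the third-person character steps into a trigger box.
; Start and End triggers call StartMovement if the platform is idle and AtBeginning or AtEnd, respectively, is true.
; StartMovement waits briefly, then a Timeline lerps location and rotation.
; The Timeline only plays forward, and neither position flag is set in these graphs.
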(event OnComponentBeginOverlap(BoxTriggerSTART)
  (params (OverlappedComponent :type Primitive%20Component%20Object%20Reference) (OtherActor :type Actor%20Object%20Reference) (OtherComp :type Primitive%20Component%20Object%20Reference) (OtherBodyIndex :type Integer) (bFromSweep :type Boolean) (SweepResult :type Hit%20Result%20Structure%20%28by%20ref%29))
  (Development|PrintString "Time to Go to the End!")
  (Utilities|Casting|CastToBP_ThirdPersonCharacter OtherActor)
  (if (not (Variables|Default|GetisPlatformMoving))
    (if (Variables|Default|GetatBeginning)
      (Development|PrintString "Calling Start Movement")
      (CallFunction|StartMovement))))

(event OnComponentBeginOverlap(BoxTriggerEND)
  (params (OverlappedComponent :type Primitive%20Component%20Object%20Reference) (OtherActor :type Actor%20Object%20Reference) (OtherComp :type Primitive%20Component%20Object%20Reference) (OtherBodyIndex :type Integer) (bFromSweep :type Boolean) (SweepResult :type Hit%20Result%20Structure%20%28by%20ref%29))
  (Development|PrintString "Time to Go to the Beginning!")
  (Utilities|Casting|CastToBP_ThirdPersonCharacter OtherActor)
  (if (not (Variables|Default|GetisPlatformMoving))
    (if (Variables|Default|GetatEnd)
      (Development|PrintString "Calling Start Movement")
      (CallFunction|StartMovement))))

(event Custom|StartMovement
  (Development|PrintString "Move Time.")
  (Variables|Default|SetisPlatformMoving true)
  (Utilities|FlowControl|Delay 2.0)
  (bind _newtrack_0 (Timeline|Timeline Play)
    (:Update
      (Transformation|SetWorldLocationAndRotation (Variables|Default|GetPlatform) (.location (Math|Transform|Lerp(Transform) (Transformation|GetWorldTransform (Variables|Default|GetStart)) (Transformation|GetWorldTransform (Variables|Default|GetEnd)) _newtrack_0)) (.rotation (Math|Transform|Lerp(Transform) (Transformation|GetWorldTransform (Variables|Default|GetStart)) (Transformation|GetWorldTransform (Variables|Default|GetEnd)) _newtrack_0)) false false))
    (:Finished
      (Variables|Default|SetisPlatformMoving false))))

(event EventBeginPlay)

(fn ConstructionScript)